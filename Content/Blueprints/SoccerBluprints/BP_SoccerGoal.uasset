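; BP_SoccerGoal is a soccer goal actor that detects when the ball enters it and respawns a new one.
; At BeginPlay it stores the location of the referenced ball as the spawn point.
; When a BP_SoccarBall overlaps its Box, it plays a hit particle effect at the goal, destroys the ball and, after a short delay, spawns a replacement at the stored location.
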(event `self.ReceiveBeginPlay`
  (bind _soccarballref (`self.SoccarBallRef`))
  (`/Engine/EditorBlueprintResources/StandardMacros.IsValid` _soccarballref
    (:`Is Valid`
      (set `self.BallSpawnLocation` (`self.K2_GetActorLocation` _soccarballref)))))

(event `self.Box.OnComponentBeginOverlap`
  (params (OverlappedComponent :type "PrimitiveComponent Object Reference") (OtherActor :type "Actor Object Reference") (OtherComp :type "PrimitiveComponent Object Reference") (OtherBodyIndex :type Integer) (bFromSweep :type Boolean) (SweepResult :type "HitResult Structure (by ref)"))
  (bind _asbp_soccar_ball (cast `/Game/Blueprints/SoccerBluprints/BP_SoccarBall` OtherActor))
  (`GameplayStatics.SpawnEmitterAtLocation` "/Game/FXVarietyPack/Particles/P_ky_hit1.P_ky_hit1" (`KismetMathLibrary.MakeVector` (.x (`SceneComponent.K2_GetComponentLocation` (`self.SoccerGoal`))) (.y (`SceneComponent.K2_GetComponentLocation` (`self.SoccerGoal`))) 200.0))
  (`self.K2_DestroyActor` _asbp_soccar_ball)
  (`KismetSystemLibrary.Delay` 2.0)
  (`|SpawnActorFromClass` "/Game/Blueprints/SoccerBluprints/BP_SoccarBall.BP_SoccarBall_C" (`KismetMathLibrary.MakeTransform` (`self.BallSpawnLocation`)) "Undefined" "OverrideRootScale" null null))

(fn `UserConstructionScript`)